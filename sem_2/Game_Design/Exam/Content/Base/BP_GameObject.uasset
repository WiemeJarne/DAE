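; Base game object Blueprint that provides visual feedback effects: color flicker, temporary scale change and timed or lasting color change.
; BeginPlay creates a dynamic material on VisualMesh and caches its Color for later restoring.
; Flicker replays a timeline blending two colors until accumulated timeline lengths reach the requested duration, then restores the cached color.
; IncreaseScale scales the root via timeline, waits, then plays it in reverse.
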(event `Flicker`
  (params (Duration :type "Float (double-precision)" :default 1.0) (Color2 :type "LinearColor Structure") (Color1 :type "LinearColor Structure" :default (struct :`R` 0.005182 :`G` 0.194618 :`B` 0.502887 :`A` 1.0)))
  (bind _returnvalue (- Duration (`self.FlickerTime`)))
  ;[1 1 1] Flicker
  (bind (_direction _flickerstate) (`Timeline|Timeline_Flicker` :`NewTime` (`KismetMathLibrary.SelectFloat` (- 1.0 _returnvalue) 0.0 (< _returnvalue 1.0)) :!via `PlayFromStart` :!label _label)
    (:`Update`
      (`MaterialInstanceDynamic.SetVectorParameterValue` (`self.VisualMeshMaterial`) "Color" (`KismetMathLibrary.LinearColorLerp` Color2 Color1 _flickerstate)))
    (:`Finished`
      (if (`self.IsFlickerTimeOver` Duration)
        (`MaterialInstanceDynamic.SetVectorParameterValue` (`self.VisualMeshMaterial`) "Color" (`self.VisualMeshColor`))
        (set `self.FlickerTime` 0.0)
        (else
          (`|ExecutionSequence`
            (:`then_0`
              (goto _label :!via `SetNewTime`))
            (:`then_1`
              (goto _label))))))))

(event `IncreaseScale`
  (params (Duration :type "Float (double-precision)") (Scale :type "Float (double-precision)"))
  ;[1 1 1] Increase Scale
  (bind (_direction _scale) (`Timeline|TimelineBodyScale` :!via `PlayFromStart` :!label _label_2)
    (:`Update`
      (`SceneComponent.SetRelativeScale3D` (`self.DefaultSceneRoot`) (`KismetMathLibrary.Conv_DoubleToVector` (+ 1.0 (* _scale Scale)))))
    (:`Finished`
      (if (`self.ComponentScaledStatus`)
        (set `self.ComponentScaledStatus` false)
        (else
          (set `self.ComponentScaledStatus` true)
          (`KismetSystemLibrary.Delay` (- Duration (* (`TimelineComponent.GetTimelineLength` (`self.TimelineBodyScale`)) 2.0)))
          (goto _label_2 :!via `ReverseFromEnd`))))))

(event `ChangeColorForDuration`
  (params (Duration :type "Float (double-precision)") (EyeColor :type "LinearColor Structure"))
  ;[1 1 1] Change Color
  (`MaterialInstanceDynamic.SetVectorParameterValue` (`self.VisualMeshMaterial`) "Color" EyeColor)
  (`KismetSystemLibrary.Delay` Duration)
  (`MaterialInstanceDynamic.SetVectorParameterValue` (`self.VisualMeshMaterial`) "Color" (`self.VisualMeshColor`)))

(event `ChangeColor`
  (params (EyeColor :type "LinearColor Structure"))
  ;[1 1 1] Change Color
  (`MaterialInstanceDynamic.SetVectorParameterValue` (`self.VisualMeshMaterial`) "Color" EyeColor))

(event `self.ReceiveBeginPlay`
  (bind _returnvalue (`PrimitiveComponent.CreateDynamicMaterialInstance` (`self.VisualMesh`) 0 null "None"))
  (bind _output_get (set `self.VisualMeshMaterial` _returnvalue))
  (bind _returnvalue_2 (`MaterialInstanceDynamic.K2_GetVectorParameterValue` _output_get "Color"))
  (set `self.VisualMeshColor` _returnvalue_2))

(event `self.ReceiveTick`
  (params (DeltaSeconds :type "Float (single-precision)")))

(fn `IsFlickerTimeOver`
  (params (FlickerTimeTotal :type "Float (double-precision)"))
  (returns (ReturnValue :type Boolean))
  (bind _output_get (set `self.FlickerTime` (+ (`self.FlickerTime`) (`TimelineComponent.GetTimelineLength` (`self.Timeline_Flicker`)))))
  (return (>= _output_get FlickerTimeTotal)))

(fn `UserConstructionScript`)