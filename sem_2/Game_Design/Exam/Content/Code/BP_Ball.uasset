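; BP_Ball is a projectile ball actor that launches along world Y at a fixed speed and recycles itself to its starting point.
; Tick accumulates time alive, but the respawn check runs only when the sphere registers a hit.
; Once the lifetime limit is reached, a hit resets the timer, moves the sphere to its saved start, then relaunches it after a short delay.
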(event `self.ReceiveBeginPlay`
  (set `self.StartPos` (`SceneComponent.K2_GetComponentLocation` (`self.Sphere`)))
  (set `MovementComponent.Velocity` (0.0 750.0 0.0) (`self.ProjectileMovement`)))

(event `self.ReceiveTick`
  (params (DeltaSeconds :type "Float (single-precision)"))
  (set `self.TimeAlive` (+ DeltaSeconds (`self.TimeAlive`))))

(event `self.Sphere.OnComponentHit`
  (params (HitComponent :type "PrimitiveComponent Object Reference") (OtherActor :type "Actor Object Reference") (OtherComp :type "PrimitiveComponent Object Reference") (NormalImpulse :type "Vector Structure") (Hit :type "HitResult Structure (by ref)"))
  (if (>= (`self.TimeAlive`) (`self.MaxAmountOfSecondsAlive`))
    (set `self.TimeAlive` 0.0)
    (`SceneComponent.K2_SetWorldLocation` (`self.Sphere`) (`self.StartPos`) false false)
    (`KismetSystemLibrary.Delay` 0.2)
    (`MovementComponent.StopMovementImmediately` (`self.ProjectileMovement`))
    (set `MovementComponent.Velocity` (0.0 750.0 0.0) (`self.ProjectileMovement`))))

(event `InputAction|StartBall`
  (params (Key :type "Key Structure")))

(fn `UserConstructionScript`)