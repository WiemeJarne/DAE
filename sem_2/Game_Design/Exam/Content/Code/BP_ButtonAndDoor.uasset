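; Puzzle actor pairing a button and a door, where hitting the button with a ball opens the door.
; BeginPlay gives the button its not-pressed material.
; When a BP_Ball hits the button, the ball is destroyed, the button switches to its pressed material, and the door component is destroyed once, guarded by a DoorHasBeenOpened flag.
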(event `self.ReceiveBeginPlay`
  (`PrimitiveComponent.SetMaterial` (`self.button`) 0 "/Game/Data/Materials/MI_NotPressedButton.MI_NotPressedButton"))

(event `self.button.OnComponentHit`
  (params (HitComponent :type "PrimitiveComponent Object Reference") (OtherActor :type "Actor Object Reference") (OtherComp :type "PrimitiveComponent Object Reference") (NormalImpulse :type "Vector Structure") (Hit :type "HitResult Structure (by ref)"))
  (bind _asbp_ball (cast `/Game/Code/BP_Ball` OtherActor))
  (`self.K2_DestroyActor` _asbp_ball)
  (`PrimitiveComponent.SetMaterial` (`self.button`) 0 "/Game/Data/Materials/MI_PressedButton.MI_PressedButton")
  (if (not (`self.DoorHasBeenOpened`))
    (`ActorComponent.K2_DestroyComponent` (`self.door`))
    (set `self.DoorHasBeenOpened` true)))

(fn `UserConstructionScript`)