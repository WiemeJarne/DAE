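; BP_NPC is an NPC Blueprint whose health steadily drains until the actor dies.
; On BeginPlay it sets an initial Behavior state, fills Health to MaxHealth and caches the HealthBar component's WBP_BodyHealthBar widget.
; Each Tick lowers Health by HealthDecay scaled by delta time, writes the value straight to the widget and destroys the actor once it drops below zero.
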(event `self.ReceiveBeginPlay`
  (`parent.ReceiveBeginPlay`)
  (set `self.Behavior` "NewEnumerator6")
  (set `self.Health` (`self.MaxHealth`))
  (bind _aswbp_body_health_bar (cast `/Game/Code/UI/WBP_BodyHealthBar` (`WidgetComponent.GetUserWidgetObject` (`self.HealthBar`))))
  (set `self.HealthBarRef` _aswbp_body_health_bar))

(event `self.ReceiveTick`
  (params (DeltaSeconds :type "Float (single-precision)"))
  (`parent.ReceiveTick` DeltaSeconds)
  (bind _output_get (set `self.Health` (- (`self.Health`) (* DeltaSeconds (`self.HealthDecay`)))))
  (set `/Game/Code/UI/WBP_BodyHealthBar.Health` _output_get (`self.HealthBarRef`))
  (if (< _output_get 0.0)
    (`self.K2_DestroyActor`)))

(fn `UserConstructionScript`
  (`parent.UserConstructionScript`))