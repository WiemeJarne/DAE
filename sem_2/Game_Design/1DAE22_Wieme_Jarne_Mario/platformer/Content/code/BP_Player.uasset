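; Player actor for a color-switching game that moves along the Y axis and reloads the current level when destroyed.
; Jump applies a capsule impulse when a downward sphere trace hits, while movement offsets location without sweep.
; ChangeMaterial cycles violet, blue, yellow and red on a frame-counted cooldown, while Force inputs spend matching pickups to set a color directly.
; Tick prints pickup and coin counts on screen as a makeshift HUD.
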(event `self.ReceiveDestroyed`
  (bind _returnvalue (`GameplayStatics.GetCurrentLevelName` true))
  (`GameplayStatics.OpenLevel` (`KismetStringLibrary.Conv_StringToName` _returnvalue)))

(event `InputAction|ChangeMaterial`
  (params (Key :type "Key Structure"))
  (:`Pressed`
    (if (<= (`self.Delay`) 0.0)
      (`self.ChangeColor`)
      (set `self.Delay` 125.0))))

(event `InputAction|ForceViolet`
  (params (Key :type "Key Structure"))
  (:`Pressed`
    (`self.ForcePurpleColorChange`)))

(event `InputAction|ForceBlue`
  (params (Key :type "Key Structure"))
  (:`Pressed`
    (`self.ForceBlueColorChangle`)))

(event `InputAction|jump`
  (params (Key :type "Key Structure"))
  (:`Pressed`
    (`self.Jump`)))

(event `InputAction|ForceYellow`
  (params (Key :type "Key Structure"))
  (:`Pressed`
    (`self.ForceYellowColorChange`)))

(event `InputAction|ForceRed`
  (params (Key :type "Key Structure"))
  (:`Pressed`
    (`self.ForceRedColorChangle`)))

(event `InputAxis|MoveRight`
  (params (AxisValue :type "Float (single-precision)"))
  (`self.Move` AxisValue))

(event `self.ReceiveBeginPlay`
  (set `self.material` (`PrimitiveComponent.GetMaterial` (`self.StaticMesh`) 0)))

(event `self.ReceiveActorBeginOverlap`
  (params (OtherActor :type "Actor Object Reference")))

(event `self.ReceiveTick`
  (params (DeltaSeconds :type "Float (single-precision)"))
  (`/Engine/EditorBlueprintResources/StandardMacros.DecrementFloat` (`self.Delay`)
    (:`  `
      (set `self.Text` "Red Pickup")
      (`self.PrintAmountOfPickups` (`self.AmountOfRedPickups`) (`self.text`))
      (set `self.Text` "Yellow Pickup")
      (`self.PrintAmountOfPickups` (`self.AmountOfYellowPickups`) (`self.text`))
      (set `self.Text` "Blue Pickup")
      (`self.PrintAmountOfPickups` (`self.AmountOfBluePickups`) (`self.text`))
      (set `self.Text` "Violet Pickup")
      (`self.PrintAmountOfPickups` (`self.AmountOfPurplePickups`) (`self.text`))
      (set `self.Text` "Coins")
      (`self.PrintAmountOfPickups` (`self.AmountOfCoins`) (`self.text`)))))

(fn `ChangeColor`
  (bind _bluematerial (`self.BlueMaterial`))
  (bind _yelowmaterial (`self.YelowMaterial`))
  (bind _redmaterial (`self.RedMaterial`))
  (bind _violetmaterial (`self.VioletMaterial`))
  (if (`self.CompareMaterials` (`self.VioletMaterial`))
    (`PrimitiveComponent.SetMaterial` (`self.StaticMesh`) 0 _bluematerial)
    (set `self.material` _bluematerial)
    (elif (`self.CompareMaterials` (`self.BlueMaterial`))
      (`PrimitiveComponent.SetMaterial` (`self.StaticMesh`) 0 _yelowmaterial)
      (set `self.material` _yelowmaterial)
      (elif (`self.CompareMaterials` (`self.YelowMaterial`))
        (`PrimitiveComponent.SetMaterial` (`self.StaticMesh`) 0 _redmaterial)
        (set `self.material` _redmaterial)
        (else
          (`PrimitiveComponent.SetMaterial` (`self.StaticMesh`) 0 _violetmaterial)
          (set `self.material` _violetmaterial))))))

(fn `CompareMaterials`
  (params (A :type "Object Object Reference"))
  (returns (ReturnValue :type Boolean))
  (return (== A (`PrimitiveComponent.GetMaterial` (`self.StaticMesh`) 0))))

(fn `ForceBlueColorChangle`
  (if (> (`self.AmountOfBluePickups`) 0)
    (bind _output_get (set `self.material` "/Game/materials/MI_Blue.MI_Blue"))
    (`PrimitiveComponent.SetMaterial` (`self.StaticMesh`) 0 _output_get)
    (`/Engine/EditorBlueprintResources/StandardMacros.DecrementInt` (`self.AmountOfBluePickups`))))

(fn `ForcePurpleColorChange`
  (if (> (`self.AmountOfPurplePickups`) 0)
    (bind _output_get (set `self.material` "/Game/materials/MI_Violet.MI_Violet"))
    (`PrimitiveComponent.SetMaterial` (`self.StaticMesh`) 0 _output_get)
    (`/Engine/EditorBlueprintResources/StandardMacros.DecrementInt` (`self.AmountOfPurplePickups`))))

(fn `ForceRedColorChangle`
  (if (> (`self.AmountOfRedPickups`) 0)
    (bind _output_get (set `self.material` "/Game/materials/MI_Red.MI_Red"))
    (`PrimitiveComponent.SetMaterial` (`self.StaticMesh`) 0 _output_get)
    (`/Engine/EditorBlueprintResources/StandardMacros.DecrementInt` (`self.AmountOfRedPickups`))))

(fn `ForceYellowColorChange`
  (if (> (`self.AmountOfYellowPickups`) 0)
    (bind _output_get (set `self.material` "/Game/materials/MI_Yellow.MI_Yellow"))
    (`PrimitiveComponent.SetMaterial` (`self.StaticMesh`) 0 _output_get)
    (`/Engine/EditorBlueprintResources/StandardMacros.DecrementInt` (`self.AmountOfYellowPickups`))))

(fn `Jump`
  (bind _returnvalue (`self.K2_GetActorLocation`))
  (bind _capsule (`self.Capsule`))
  (bind (_outhits _returnvalue_2) (`KismetSystemLibrary.SphereTraceMulti` _returnvalue (- _returnvalue (`KismetMathLibrary.MakeVector` 0.0 0.0 (`CapsuleComponent.CapsuleHalfHeight` _capsule))) (/ (`CapsuleComponent.CapsuleRadius` _capsule) 2.0) "TraceTypeQuery1"))
  (if _returnvalue_2
    (`PrimitiveComponent.AddImpulse` (`self.Capsule`) (`KismetMathLibrary.MakeVector` 0.0 0.0 (`self.JumpForce`)) "None" true)))

(fn `Move`
  (params (B :type "Float (double-precision)"))
  (`self.K2_SetActorLocation` (+ (* (* (`KismetMathLibrary.MakeVector` 0.0 (`self.WalkSpeed`)) B) (`GameplayStatics.GetWorldDeltaSeconds`)) (`self.K2_GetActorLocation`))))

(fn `PrintAmountOfPickups`
  (params (InInt :type Integer) (A :type String))
  (locals (AmountOfPickups :type Integer) (ColorPickup :type String))
  (set `local.AmountOfPickups` InInt)
  (set `local.ColorPickup` A)
  (if (`KismetStringLibrary.EqualEqual_StrStr` (`local.ColorPickup`) "Violet Pickup")
    (`KismetSystemLibrary.PrintString` (`KismetStringLibrary.Concat_StrStr` (`local.ColorPickup`) ": " (`KismetStringLibrary.Conv_IntToString` (`local.AmountOfPickups`)) "  (press 1)") true false (struct :`A` 1.0) 0.0)
    (elif (`KismetStringLibrary.EqualEqual_StrStr` (`local.ColorPickup`) "Blue Pickup")
      (`KismetSystemLibrary.PrintString` (`KismetStringLibrary.Concat_StrStr` (`local.ColorPickup`) ": " (`KismetStringLibrary.Conv_IntToString` (`local.AmountOfPickups`)) "  (press 2)") true false (struct :`A` 1.0) 0.0)
      (elif (`KismetStringLibrary.EqualEqual_StrStr` (`local.ColorPickup`) "Yellow Pickup")
        (`KismetSystemLibrary.PrintString` (`KismetStringLibrary.Concat_StrStr` (`local.ColorPickup`) ": " (`KismetStringLibrary.Conv_IntToString` (`local.AmountOfPickups`)) "  (press 3)") true false (struct :`A` 1.0) 0.0)
        (elif (`KismetStringLibrary.EqualEqual_StrStr` (`local.ColorPickup`) "Red Pickup")
          (`KismetSystemLibrary.PrintString` (`KismetStringLibrary.Concat_StrStr` (`local.ColorPickup`) ": " (`KismetStringLibrary.Conv_IntToString` (`local.AmountOfPickups`)) "  (press 4)") true false (struct :`A` 1.0) 0.0)
          (else
            (`KismetSystemLibrary.PrintString` (`KismetStringLibrary.Concat_StrStr` (`local.ColorPickup`) ": " (`KismetStringLibrary.Conv_IntToString` (`local.AmountOfPickups`))) true false (struct :`A` 1.0) 0.0)))))))

(fn `UserConstructionScript`)