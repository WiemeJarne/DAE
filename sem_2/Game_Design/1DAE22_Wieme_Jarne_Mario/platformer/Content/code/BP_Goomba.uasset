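; BP_Goomba is a Mario-style enemy that patrols back and forth along the Y axis.
; On BeginPlay it detaches two target components and places them half the control-point distance to either side of its start.
; Tick moves it by direction and speed, reversing whenever it passes a target.
; Overlapping DangerSpot destroys BP_Player, while a player touching WeakSpot squashes and stops the Goomba, then destroys it after a short delay.
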(event `self.ReceiveBeginPlay`
  (`SceneComponent.K2_DetachFromComponent` (`self.Target_Right`) "KeepWorld" "KeepWorld" "KeepWorld" true)
  (`SceneComponent.K2_DetachFromComponent` (`self.Target_Left`) "KeepWorld" "KeepWorld" "KeepWorld" true)
  (`self.ChangeTargetRightLocation`)
  (`self.ChangeTargetLeftLocation`))

(event `self.ReceiveTick`
  (params (DeltaSeconds :type "Float (single-precision)"))
  (`self.K2_SetActorLocation` (`self.CalculateNewLocation` DeltaSeconds))
  (if (or (and (`self.IsMovingRight`) (`self.IsPastRightTarget`)) (and (`self.IsMovingLeft`) (`self.IsPatRightTarget`)))
    (`self.InvertDirection`)))

(event `self.DangerSpot.OnComponentBeginOverlap`
  (params (OverlappedComponent :type "PrimitiveComponent Object Reference") (OtherActor :type "Actor Object Reference") (OtherComp :type "PrimitiveComponent Object Reference") (OtherBodyIndex :type Integer) (bFromSweep :type Boolean) (SweepResult :type "HitResult Structure (by ref)"))
  (bind _asbp_player (cast `/Game/code/BP_Player` OtherActor))
  (`self.K2_DestroyActor` _asbp_player))

(event `self.WeakSpot.OnComponentBeginOverlap`
  (params (OverlappedComponent :type "PrimitiveComponent Object Reference") (OtherActor :type "Actor Object Reference") (OtherComp :type "PrimitiveComponent Object Reference") (OtherBodyIndex :type Integer) (bFromSweep :type Boolean) (SweepResult :type "HitResult Structure (by ref)"))
  (cast `/Game/code/BP_Player` OtherActor)
  (`self.SetActorScale3D` (1.0 1.0 0.5))
  (set `self.MoveDirection` (0.0 0.0 0.0))
  (`KismetSystemLibrary.Delay` 0.5)
  (`self.K2_DestroyActor`))

(fn `CalculateNewLocation`
  (params (A :type "Float (double-precision)"))
  (returns (ReturnValue :type "Vector Structure"))
  (return (+ (`self.K2_GetActorLocation`) (* (`self.MoveDirection`) (* A (`self.MoveSpeed`))))))

(fn `ChangeTargetLeftLocation`
  (`SceneComponent.K2_SetRelativeLocation` (`self.Target_Left`) (- (`self.K2_GetActorLocation`) (`KismetMathLibrary.MakeVector` 0.0 (/ (`self.DistanceBetweenControlPoints`) 2.0))) false false))

(fn `ChangeTargetRightLocation`
  (`SceneComponent.K2_SetRelativeLocation` (`self.Target_Right`) (+ (`self.K2_GetActorLocation`) (`KismetMathLibrary.MakeVector` 0.0 (/ (`self.DistanceBetweenControlPoints`) 2.0))) false false))

(fn `InvertDirection`
  (set `self.MoveDirection` (* (`self.MoveDirection`) -1.0)))

(fn `IsMovingLeft`
  (returns (ReturnValue :type Boolean))
  (bind (_movedirection_x _movedirection_y) (`KismetMathLibrary.BreakVector` (`self.MoveDirection`)))
  (return (< _movedirection_y 0.0)))

(fn `IsMovingRight`
  (returns (ReturnValue :type Boolean))
  (bind (_movedirection_x _movedirection_y) (`KismetMathLibrary.BreakVector` (`self.MoveDirection`)))
  (return (> _movedirection_y 0.0)))

(fn `IsPastRightTarget`
  (returns (ReturnValue :type Boolean))
  (bind (_returnvalue_x _returnvalue_y) (`KismetMathLibrary.BreakVector` (`self.K2_GetActorLocation`)))
  (bind (_returnvalue_x_2 _returnvalue_y_2) (`KismetMathLibrary.BreakVector` (`SceneComponent.K2_GetComponentLocation` (`self.Target_Right`))))
  (return (> _returnvalue_y _returnvalue_y_2)))

(fn `IsPatRightTarget`
  (returns (ReturnValue :type Boolean))
  (bind (_returnvalue_x _returnvalue_y) (`KismetMathLibrary.BreakVector` (`self.K2_GetActorLocation`)))
  (bind (_returnvalue_x_2 _returnvalue_y_2) (`KismetMathLibrary.BreakVector` (`SceneComponent.K2_GetComponentLocation` (`self.Target_Left`))))
  (return (< _returnvalue_y _returnvalue_y_2)))

(fn `UserConstructionScript`)