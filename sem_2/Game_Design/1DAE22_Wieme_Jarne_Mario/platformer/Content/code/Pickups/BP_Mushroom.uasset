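; BP_Mushroom is a moving mushroom pickup that the player collects by touching it.
; Each Tick it moves without sweep along MoveDirection, scaled by MoveSpeed and delta time through CalculateNewLocation.
; When its Sphere overlaps a BP_Player, it prints a pickup message and destroys itself, granting nothing.
; An IncrementAmountOfCoins function is defined but never called in this Blueprint.
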(event `self.ReceiveBeginPlay`)

(event `self.ReceiveActorBeginOverlap`
  (params (OtherActor :type "Actor Object Reference")))

(event `self.ReceiveTick`
  (params (DeltaSeconds :type "Float (single-precision)"))
  (`self.K2_SetActorLocation` (`self.CalculateNewLocation` DeltaSeconds)))

(event `self.Sphere.OnComponentBeginOverlap`
  (params (OverlappedComponent :type "PrimitiveComponent Object Reference") (OtherActor :type "Actor Object Reference") (OtherComp :type "PrimitiveComponent Object Reference") (OtherBodyIndex :type Integer) (bFromSweep :type Boolean) (SweepResult :type "HitResult Structure (by ref)"))
  (cast `/Game/code/BP_Player` OtherActor)
  (`KismetSystemLibrary.PrintString` "You picked up a mushroom" true true (struct :`A` 1.0))
  (`self.K2_DestroyActor`))

(fn `CalculateNewLocation`
  (params (A :type "Float (double-precision)"))
  (returns (ReturnValue :type "Vector Structure"))
  (return (+ (`self.K2_GetActorLocation`) (* (`self.MoveDirection`) (* A (`self.MoveSpeed`))))))

(fn `IncrementAmountOfCoins`
  (params (self2 :type "/Game/code/BP_Player Object Reference") (self3 :type "/Game/code/BP_Player Object Reference"))
  (set `/Game/code/BP_Player.AmountOfCoins` (+ (`/Game/code/BP_Player.AmountOfCoins` self3) 1) self2))

(fn `UserConstructionScript`)