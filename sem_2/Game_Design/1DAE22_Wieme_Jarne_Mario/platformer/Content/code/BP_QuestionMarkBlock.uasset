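; BP_QuestionMarkBlock is a question mark block that releases a BP_Mushroom when the player overlaps its Box.
; The overlap casts to BP_Player, moves the root up, spawns the half-scale mushroom, then after a short delay lowers the root slightly past its start.
; HasActivated limits it to one use, but is only set after these latent steps finish.
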(event `self.Box.OnComponentBeginOverlap`
  (params (OverlappedComponent :type "PrimitiveComponent Object Reference") (OtherActor :type "Actor Object Reference") (OtherComp :type "PrimitiveComponent Object Reference") (OtherBodyIndex :type Integer) (bFromSweep :type Boolean) (SweepResult :type "HitResult Structure (by ref)"))
  (bind _defaultsceneroot (`self.DefaultSceneRoot`))
  (bind _defaultsceneroot_2 (`self.DefaultSceneRoot`))
  (bind (_returnvalue_location _returnvalue_rotation) (`KismetMathLibrary.BreakTransform` (`SceneComponent.GetRelativeTransform` _defaultsceneroot)))
  (bind (_returnvalue_location_2 _returnvalue_rotation_2) (`KismetMathLibrary.BreakTransform` (`SceneComponent.GetRelativeTransform` _defaultsceneroot_2)))
  (cast `/Game/code/BP_Player` OtherActor)
  (if (not (`self.HasActivated`))
    (`KismetSystemLibrary.MoveComponentTo` _defaultsceneroot_2 (+ _returnvalue_location_2 (0.0 0.0 40.0)) _returnvalue_rotation_2 false false 0.1)
    (`|SpawnActorFromClass` "/Game/code/Pickups/BP_Mushroom.BP_Mushroom_C" (`KismetMathLibrary.MakeTransform` (- (`self.K2_GetActorLocation`) (0.0 10.0 -40.0)) (struct) (0.5 0.5 0.5)) "Undefined" "OverrideRootScale" null null)
    (`KismetSystemLibrary.Delay` 0.5)
    (`KismetSystemLibrary.MoveComponentTo` _defaultsceneroot (+ _returnvalue_location (0.0 0.0 -45.0)) _returnvalue_rotation false false 0.1)
    (set `self.HasActivated` true)))

(fn `UserConstructionScript`)