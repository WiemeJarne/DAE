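; BP_CoinPickup is a coin pickup that adds to the player's coin count when overlapped.
; On BeginPlay it casts the first player pawn to BP_Player and caches the reference.
; Any actor overlap, with no check on the overlapping actor, prints a brief pickup message, increments AmountOfCoins on that cached player and destroys the coin.
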(event `self.ReceiveBeginPlay`
  (bind _asbp_player (cast `/Game/code/BP_Player` (`GameplayStatics.GetPlayerPawn` 0)))
  (set `self.player` _asbp_player))

(event `self.ReceiveActorBeginOverlap`
  (params (OtherActor :type "Actor Object Reference"))
  (`KismetSystemLibrary.PrintString` "You picked up a coin" true true (struct :`A` 1.0) 0.5)
  (`self.IncrementAmountOfCoins`)
  (`self.K2_DestroyActor`))

(fn `IncrementAmountOfCoins`
  (`/Engine/EditorBlueprintResources/StandardMacros.IncrementInt` (`/Game/code/BP_Player.AmountOfCoins` (`self.player`))))

(fn `UserConstructionScript`)