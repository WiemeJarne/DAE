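; A violet color-matched platform that is solid only while the player's material matches its color.
; On BeginPlay it caches the BP_Player pawn, then every Tick compares the player's material to the mesh's current material.
; The comparison is by name, stripping "Translucent" from the platform's material string.
; A match applies the opaque violet material and enables collision; otherwise the platform turns translucent with no collision.
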(event `self.ReceiveActorBeginOverlap`
  (params (OtherActor :type "Actor Object Reference")))

(event `self.ReceiveBeginPlay`
  (bind _asbp_player (cast `/Game/code/BP_Player` (`GameplayStatics.GetPlayerPawn` 0)))
  (set `self.Player` _asbp_player))

(event `self.ReceiveTick`
  (params (DeltaSeconds :type "Float (single-precision)"))
  (if (`self.CompareMaterials` (`/Game/code/BP_Player.material` (`self.Player`)) (`PrimitiveComponent.GetMaterial` (`self.StaticMesh`) 0))
    (`self.MakePlatformSolid`)
    (else
      (`self.MakePlatFormTranslucent`))))

(fn `CompareMaterials`
  (params (InObj :type "Object Object Reference") (InObj2 :type "Object Object Reference"))
  (returns (ReturnValue :type Boolean))
  (return (`KismetStringLibrary.EqualEqual_StrStr` (`KismetStringLibrary.Replace` (`KismetStringLibrary.Conv_ObjectToString` InObj2) "Translucent") (`KismetStringLibrary.Conv_ObjectToString` InObj))))

(fn `MakePlatformSolid`
  (`PrimitiveComponent.SetMaterial` (`self.StaticMesh`) 0 "/Game/materials/MI_Violet.MI_Violet")
  (`PrimitiveComponent.SetCollisionEnabled` (`self.StaticMesh`) "QueryAndPhysics"))

(fn `MakePlatFormTranslucent`
  (`PrimitiveComponent.SetMaterial` (`self.StaticMesh`) 0 "/Game/materials/MI_TranslucentViolet.MI_TranslucentViolet")
  (`PrimitiveComponent.SetCollisionEnabled` (`self.StaticMesh`) "NoCollision"))

(fn `UserConstructionScript`)