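; BP_Projectile is a projectile Blueprint that returns to its starting point after too many impacts.
; On BeginPlay it stores the Sphere component's world location as StartPos.
; Each Sphere hit increments a counter, and once that exceeds MaxHits the counter resets and the Sphere moves back to StartPos without sweeping, rather than being destroyed.
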(event `self.ReceiveBeginPlay`
  (set `self.StartPos` (`SceneComponent.K2_GetComponentLocation` (`self.Sphere`))))

(event `self.Sphere.OnComponentHit`
  (params (HitComponent :type "PrimitiveComponent Object Reference") (OtherActor :type "Actor Object Reference") (OtherComp :type "PrimitiveComponent Object Reference") (NormalImpulse :type "Vector Structure") (Hit :type "HitResult Structure (by ref)"))
  (bind _result (`/Engine/EditorBlueprintResources/StandardMacros.IncrementInt` (`self.AmountOfHit`))
    (:`  `
      (if (> _result (`self.MaxHits`))
        (set `self.AmountOfHit` 0)
        (`SceneComponent.K2_SetWorldLocation` (`self.Sphere`) (`self.StartPos`) false false)))))

(fn `UserConstructionScript`)