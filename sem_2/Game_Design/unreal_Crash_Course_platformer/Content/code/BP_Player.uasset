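; BP_Player is a player character that moves along the Y axis, jumps, and prints its Score on screen every tick.
; MoveRight input offsets the location by WalkSpeed scaled by frame time, without sweeping.
; Jump applies an upward velocity-change impulse to the Capsule only when a downward sphere trace reports a hit, acting as a ground check.
; Destruction reloads the current level.
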(event `self.ReceiveDestroyed`
  (bind _returnvalue (`GameplayStatics.GetCurrentLevelName` true))
  (`GameplayStatics.OpenLevel` (`KismetStringLibrary.Conv_StringToName` _returnvalue)))

(event `InputAction|jump`
  (params (Key :type "Key Structure"))
  (:`Pressed`
    (`self.Jump`)))

(event `InputAxis|MoveRight`
  (params (AxisValue :type "Float (single-precision)"))
  (`self.Move` AxisValue))

(event `self.ReceiveTick`
  (params (DeltaSeconds :type "Float (single-precision)"))
  (`KismetSystemLibrary.PrintString` (`KismetStringLibrary.Concat_StrStr` "Score: " (`KismetStringLibrary.Conv_IntToString` (`self.Score`))) true true (struct :`G` 0.66 :`B` 1.0 :`A` 1.0) 0.0))

(fn `Jump`
  (bind _returnvalue (`self.K2_GetActorLocation`))
  (bind _capsule (`self.Capsule`))
  (bind (_outhits _returnvalue_2) (`KismetSystemLibrary.SphereTraceMulti` _returnvalue (- _returnvalue (`KismetMathLibrary.MakeVector` 0.0 0.0 (`CapsuleComponent.CapsuleHalfHeight` _capsule))) (/ (`CapsuleComponent.CapsuleRadius` _capsule) 2.0) "TraceTypeQuery1"))
  (if _returnvalue_2
    (`PrimitiveComponent.AddImpulse` (`self.Capsule`) (`KismetMathLibrary.MakeVector` 0.0 0.0 (`self.JumpForce`)) "None" true)))

(fn `Move`
  (params (B :type "Float (double-precision)"))
  (`self.K2_SetActorLocation` (+ (* (* (`KismetMathLibrary.MakeVector` 0.0 (`self.WalkSpeed`)) B) (`GameplayStatics.GetWorldDeltaSeconds`)) (`self.K2_GetActorLocation`))))

(fn `UserConstructionScript`)