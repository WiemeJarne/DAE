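; BP_Ball is a projectile ball actor that travels along a world axis and destroys itself after a set lifetime.
; On BeginPlay it stores its start position and calls DetermineAndSetVelocity, which sorts the Ball's world yaw into quadrant ranges to set ProjectileMovement velocity along positive or negative X or Y.
; Tick accumulates time alive and destroys the actor once it reaches MaxAmountOfSecondsAlive.
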(event `self.ReceiveBeginPlay`
  (set `self.StartPos` (`SceneComponent.K2_GetComponentLocation` (`self.ball`)))
  (`self.DetermineAndSetVelocity`))

(event `self.ReceiveTick`
  (params (DeltaSeconds :type "Float (single-precision)"))
  (set `self.TimeAlive` (+ DeltaSeconds (`self.TimeAlive`)))
  (if (>= (`self.TimeAlive`) (`self.MaxAmountOfSecondsAlive`))
    (`self.K2_DestroyActor`)))

(fn `DetermineAndSetVelocity`
  (bind (_returnvalue_roll _returnvalue_pitch _returnvalue_yaw) (`KismetMathLibrary.BreakRotator` (`SceneComponent.K2_GetComponentRotation` (`self.ball`))))
  (bind (_returnvalue_roll_2 _returnvalue_pitch_2 _returnvalue_yaw_2) (`KismetMathLibrary.BreakRotator` (`SceneComponent.K2_GetComponentRotation` (`self.ball`))))
  (bind (_returnvalue_roll_3 _returnvalue_pitch_3 _returnvalue_yaw_3) (`KismetMathLibrary.BreakRotator` (`SceneComponent.K2_GetComponentRotation` (`self.ball`))))
  (bind (_returnvalue_roll_4 _returnvalue_pitch_4 _returnvalue_yaw_4) (`KismetMathLibrary.BreakRotator` (`SceneComponent.K2_GetComponentRotation` (`self.ball`))))
  (if (and (>= _returnvalue_yaw_3 0.0) (< _returnvalue_yaw_3 89.0))
    (set `MovementComponent.Velocity` (`KismetMathLibrary.MakeVector` (`self.Velocity`)) (`self.ProjectileMovement`))
    (elif (and (>= _returnvalue_yaw_4 89.0) (< _returnvalue_yaw_4 180.0))
      (set `MovementComponent.Velocity` (`KismetMathLibrary.MakeVector` 0.0 (`self.Velocity`)) (`self.ProjectileMovement`))
      (elif (and (<= _returnvalue_yaw 0.0) (> _returnvalue_yaw -90.0))
        (set `MovementComponent.Velocity` (`KismetMathLibrary.MakeVector` 0.0 (* -1 (`self.Velocity`))) (`self.ProjectileMovement`))
        (elif (and (<= _returnvalue_yaw_2 -90.0) (> _returnvalue_yaw_2 -180.0))
          (set `MovementComponent.Velocity` (`KismetMathLibrary.MakeVector` (* -1 (`self.Velocity`))) (`self.ProjectileMovement`)))))))

(fn `UserConstructionScript`)