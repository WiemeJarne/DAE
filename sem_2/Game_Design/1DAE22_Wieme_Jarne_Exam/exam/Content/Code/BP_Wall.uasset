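; BP_Wall is a wall actor whose health drains over time until it is destroyed.
; On BeginPlay it sets Health to MaxHealth and caches the WBP_BodyHealthBar widget from its HealthBar component.
; Each Tick, CalculateHealth subtracts HealthDecay scaled by delta time, the result is pushed to the health bar, and the actor destroys itself once Health drops below zero.
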(event `self.ReceiveBeginPlay`
  (set `self.Health` (`self.MaxHealth`))
  (bind _aswbp_body_health_bar (cast `/Game/Code/UI/WBP_BodyHealthBar` (`WidgetComponent.GetUserWidgetObject` (`self.HealthBar`))))
  (set `self.HealthBarRef` _aswbp_body_health_bar))

(event `self.ReceiveTick`
  (params (DeltaSeconds :type "Float (single-precision)"))
  (bind _output_get (set `self.Health` (`self.CalculateHealth` DeltaSeconds)))
  (set `/Game/Code/UI/WBP_BodyHealthBar.Health` _output_get (`self.HealthBarRef`))
  (if (< _output_get 0.0)
    (`self.K2_DestroyActor`)))

(fn `CalculateHealth`
  (params (A :type "Float (double-precision)"))
  (returns (ReturnValue :type "Float (double-precision)"))
  (return (- (`self.Health`) (* A (`self.HealthDecay`)))))

(fn `UserConstructionScript`)