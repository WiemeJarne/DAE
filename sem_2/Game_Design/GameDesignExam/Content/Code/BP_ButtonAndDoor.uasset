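; BP_ButtonAndDoor is an actor with a button and a door, where shooting the button opens the door.
; BeginPlay applies the unpressed button and door materials.
; When a BP_Projectile hits the Button, it switches to the pressed material and, the first time only, destroys the Door component and sets IsDoorOpen, so the door opens permanently.
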(event `self.ReceiveBeginPlay`
  (`PrimitiveComponent.SetMaterial` (`self.button`) 0 "/Game/Data/Materials/MI_NotPressedButton.MI_NotPressedButton")
  (`PrimitiveComponent.SetMaterial` (`self.door`) 0 "/Game/Data/Materials/MI_Door.MI_Door"))

(event `self.button.OnComponentHit`
  (params (HitComponent :type "PrimitiveComponent Object Reference") (OtherActor :type "Actor Object Reference") (OtherComp :type "PrimitiveComponent Object Reference") (NormalImpulse :type "Vector Structure") (Hit :type "HitResult Structure (by ref)"))
  (cast `/Game/Code/BP_Projectile` OtherActor)
  (`PrimitiveComponent.SetMaterial` (`self.button`) 0 "/Game/Data/Materials/MI_PressedButton.MI_PressedButton")
  (if (not (`self.IsDoorOpen`))
    (`ActorComponent.K2_DestroyComponent` (`self.door`))
    (set `self.IsDoorOpen` true)))

(fn `UserConstructionScript`)