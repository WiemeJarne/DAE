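; Player character that carries a spawned weapon, fires it and counts the shots taken.
; On BeginPlay it spawns BP_Weapon attached to the mesh's WeaponSocket, detaches the camera to a fixed point above the world origin and creates the HUD.
; Shooting stays gated by CanShoot, which the HUD's EnemiesAreInvisible event sets to true.
; Shoot fires the weapon and increments AmountOfShots, which a separate event resets.
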(event `self.ReceiveBeginPlay`
  (bind _camera1 (`self.Camera1`))
  (`parent.ReceiveBeginPlay`)
  (`|ExecutionSequence`
    (:`then_0`
      ;[1 1 1] spawn weapon
      (bind _returnvalue (`|SpawnActorFromClass` "/Game/Blueprints/BP_Weapon.BP_Weapon_C" (`SceneComponent.K2_GetComponentToWorld` (`self.WeaponSocket`)) "Undefined" "OverrideRootScale" null null))
      (bind _output_get (set `self.WeaponOjbectReference` _returnvalue))
      ;[1 1 1] attach weapon to WeaponSocket
      (`self.K2_AttachToComponent` _output_get (`self.Mesh`) "WeaponSocket" "SnapToTarget" "SnapToTarget" "KeepRelative" true)
      ;[1 1 1] detach camera and set camera location to world origin
      (`SceneComponent.K2_DetachFromComponent` _camera1 "KeepRelative" "KeepRelative" "KeepRelative" true)
      (`SceneComponent.K2_SetWorldLocation` _camera1 (0.0 0.0 750.0) false false))
    (:`then_1`
      ;[1 1 1] setup HUD
      (bind _returnvalue_2 (`|CreateWidget` "/Game/UI/HUD.HUD_C"))
      (bind _output_get_2 (set `self.HUDReference` _returnvalue_2))
      (`UserWidget.AddToViewport` _output_get_2 0)
      (add `/Game/UI/HUD.EnemiesAreInvisible` (`self.HUDReference`) (delegate `SetCanShoot`)))))

(event `SetCanShoot`
  (set `self.CanShoot` true))

(event `Shoot`
  (if (`self.CanShoot`)
    (bind _weaponojbectreference (`self.WeaponOjbectReference`)
      (:`then`
        (`/Game/Blueprints/BP_Weapon.Fire` _weaponojbectreference)
        (`/Engine/EditorBlueprintResources/StandardMacros.IncrementInt` (`self.AmountOfShots`)))
      (:`else`))))

(event `ResetAmountOfShots`
  (set `self.AmountOfShots` 0))

(fn `UserConstructionScript`
  (`parent.UserConstructionScript`))