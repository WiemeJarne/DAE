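; BP_Laser is a laser actor with an energy pool that drains when it hits BP_Wall actors.
; On BeginPlay it fills its energy and creates a dynamic material instance for the Laser component.
; Each wall hit subtracts that wall's DamageValue, then either destroys the actor at zero or below or updates the color.
; The color parameter lerps from green to red as energy falls, showing remaining energy.
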(event `self.ReceiveBeginPlay`
  (set `self.EnergyAmount` (`self.MaxEnergyAmount`))
  (bind _returnvalue (`PrimitiveComponent.CreateDynamicMaterialInstance` (`self.Laser`) 0 null "None"))
  (bind _output_get (set `self.LaserMaterialInstance` _returnvalue))
  (`MaterialInstanceDynamic.SetVectorParameterValue` _output_get "color" (`KismetMathLibrary.LinearColorLerp` (struct :`R` 1.0 :`A` 1.0) (struct :`G` 1.0 :`A` 1.0) (/ (`KismetMathLibrary.Conv_IntToDouble` (`self.EnergyAmount`)) (`KismetMathLibrary.Conv_IntToDouble` (`self.MaxEnergyAmount`))))))

(event `self.ReceiveActorBeginOverlap`
  (params (OtherActor :type "Actor Object Reference")))

(event `self.ReceiveTick`
  (params (DeltaSeconds :type "Float (single-precision)")))

(event `self.Collision.OnComponentHit`
  (params (HitComponent :type "PrimitiveComponent Object Reference") (OtherActor :type "Actor Object Reference") (OtherComp :type "PrimitiveComponent Object Reference") (NormalImpulse :type "Vector Structure") (Hit :type "HitResult Structure (by ref)"))
  (bind _asbp_wall (cast `/Game/Blueprints/BP_Wall` OtherActor))
  (set `self.EnergyAmount` (- (`self.EnergyAmount`) (`/Game/Blueprints/BP_Wall.DamageValue` _asbp_wall)))
  ;[1 1 1] check if the EnergyAmount is below or equal to zero and destroy if true
  (if (<= (`self.EnergyAmount`) 0)
    (`self.K2_DestroyActor`)
    (else
      (bind _lasermaterialinstance (`self.LaserMaterialInstance`)
        (:`then`
          (`MaterialInstanceDynamic.SetVectorParameterValue` _lasermaterialinstance "color" (`KismetMathLibrary.LinearColorLerp` (struct :`R` 1.0 :`A` 1.0) (struct :`G` 1.0 :`A` 1.0) (/ (`KismetMathLibrary.Conv_IntToDouble` (`self.EnergyAmount`)) (`KismetMathLibrary.Conv_IntToDouble` (`self.MaxEnergyAmount`))))))
        (:`else`)))))

(fn `UserConstructionScript`)