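; BPC_Health is a health component that tracks an actor's integer health and signals when it dies.
; Health resets to the maximum on BeginPlay, and GetHealthPercentage and IsDead derive the current state from it.
; DoDamage clamps the reduced health between zero and the maximum, calls the OnDeath dispatcher only when that hit actually lowered health to zero, and returns whether the owner is dead.
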(event `ResetHealth`
  (set `self.CurrentHealth` (`self.MaxHealth`)))

(event `self.ReceiveBeginPlay`
  (`self.ResetHealth`))

(fn `DoDamage`
  (params (Amount :type Integer))
  (returns (IsDead :type Boolean))
  (bind _isdead (`self.IsDead`))
  (set `self.HealthBeforeDamage` (`self.CurrentHealth`))
  (bind _output_get (set `self.CurrentHealth` (`KismetMathLibrary.Clamp` (- (`self.CurrentHealth`) Amount) 0 (`self.MaxHealth`))))
  (if (and (> (`self.HealthBeforeDamage`) _output_get) _isdead)
    (`self.OnDeath`))
  (return _isdead))

(fn `GetHealthPercentage`
  (returns (HealthPercentage :type "Float (double-precision)"))
  (return (/ (`KismetMathLibrary.Conv_IntToDouble` (`self.CurrentHealth`)) (`KismetMathLibrary.Conv_IntToDouble` (`self.MaxHealth`)))))

(fn `IsDead`
  (returns (IsDead :type Boolean))
  (return (== (`self.GetHealthPercentage`) 0.0)))