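; BP_Weapon is a laser weapon that spawns a BP_Laser at its fire socket and shows a bouncing beam preview.
; Fire spawns a new laser only while no previous one is valid, and Tick hides the beam while that laser exists.
; Otherwise, Tick line-traces forward, mirrors the direction off the hit normal for a second trace, and feeds both hits into the Beam component's parameters.
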(event `self.ReceiveBeginPlay`
  (bind _beam (`self.Beam`))
  (`FXSystemComponent.SetVectorParameter` _beam "BeamStart" (`SceneComponent.K2_GetComponentLocation` _beam)))

(event `self.ReceiveTick`
  (params (DeltaSeconds :type "Float (single-precision)"))
  (bind _beam (`self.Beam`))
  (bind _firesocket (`self.FireSocket`))
  (bind _returnvalue (`SceneComponent.K2_GetComponentLocation` _firesocket))
  (`self.LaserObjectRef`
    (:`then`
      (`SceneComponent.SetVisibility` _beam false false))
    (:`else`
      (`SceneComponent.SetVisibility` _beam true false)
      (bind _outhits (`KismetSystemLibrary.LineTraceMultiForObjects` :`Start` _returnvalue :`End` (+ _returnvalue (* (`SceneComponent.GetForwardVector` _firesocket) (`self.LaserLenght`))) :`ObjectTypes` (`|MakeArray` "ObjectTypeQuery1" "ObjectTypeQuery2" :!type "EObjectTypeQuery Enum") :`TraceColor` (struct :`R` 30.0 :`A` 1.0) :`TraceHitColor` (struct :`A` 1.0)))
      (for _array_element _outhits
        (bind (_bblockinghit _binitialoverlap _time _distance _location _impactpoint _normal _impactnormal _physmat _hitactor) (`GameplayStatics.BreakHitResult` _array_element))
        (`/Engine/EditorBlueprintResources/StandardMacros.IsValid` _hitactor
          (:`Is Valid`
            (break))))
      (`FXSystemComponent.SetFloatParameter` (`self.Beam`) "BeamDistance" _distance)
      (`FXSystemComponent.SetVectorParameter` (`self.Beam`) "Beam2Start" _location)
      (bind _outhits_2 (`KismetSystemLibrary.LineTraceMultiForObjects` :`Start` (+ _location (1.0 1.0 0.0)) :`End` (+ _location (* (`KismetMathLibrary.MirrorVectorByNormal` (`SceneComponent.GetForwardVector` (`self.FireSocket`)) _normal) (`self.LaserLenght`))) :`ObjectTypes` (`|MakeArray` "ObjectTypeQuery1" "ObjectTypeQuery2" :!type "EObjectTypeQuery Enum") :`TraceColor` (struct :`R` 30.0 :`A` 1.0) :`TraceHitColor` (struct :`A` 1.0)))
      (for _array_element_2 _outhits_2
        (bind (_bblockinghit_2 _binitialoverlap_2 _time_2 _distance_2 _location_2 _impactpoint_2 _normal_2 _impactnormal_2 _physmat_2 _hitactor_2) (`GameplayStatics.BreakHitResult` _array_element_2))
        (`/Engine/EditorBlueprintResources/StandardMacros.IsValid` _hitactor_2
          (:`Is Valid`
            (break))))
      (`FXSystemComponent.SetVectorParameter` (`self.Beam`) "target" _impactpoint_2))))

(event `Fire`
  (`self.LaserObjectRef`
    (:`then`)
    (:`else`
      (bind _returnvalue (`|SpawnActorFromClass` "/Game/Blueprints/BP_Laser.BP_Laser_C" (`SceneComponent.K2_GetComponentToWorld` (`self.FireSocket`)) "Undefined" "OverrideRootScale" null null))
      (set `self.LaserObjectRef` _returnvalue))))

(fn `UserConstructionScript`)