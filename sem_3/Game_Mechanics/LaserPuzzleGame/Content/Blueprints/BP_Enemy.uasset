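; BP_Enemy is an enemy actor that takes damage from lasers and dies when its health component runs out.
; Capsule overlaps with a BP_Laser pass that laser's damage amount to the Health component.
; On death it plays an attached Wilhelm scream, fires the EnemyDied call and destroys itself.
; The construction script creates a dynamic material instance to tint the mesh body with EnemyColor.
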(event `self.Health.OnDeath`
  (`GameplayStatics.SpawnSoundAttached` "/Game/Audio/WilhelmScream.WilhelmScream" (`self.Mesh`) "None" (0.0 0.0 0.0) (struct) "KeepRelativeOffset" false 1.0 1.0 0.0 null null)
  (`self.EnemyDied`)
  (`self.K2_DestroyActor`))

(event `self.CapsuleComponent.OnComponentBeginOverlap`
  (params (OverlappedComponent :type "PrimitiveComponent Object Reference") (OtherActor :type "Actor Object Reference") (OtherComp :type "PrimitiveComponent Object Reference") (OtherBodyIndex :type Integer) (bFromSweep :type Boolean) (SweepResult :type "HitResult Structure (by ref)"))
  (bind _asbp_laser (cast `/Game/Blueprints/BP_Laser` OtherActor))
  (`HealthComponent.DoDamage` (`self.Health`) (`/Game/Blueprints/BP_Laser.AmountOfDamage` _asbp_laser)))

(fn `UserConstructionScript`
  (`parent.UserConstructionScript`)
  (bind _returnvalue (`PrimitiveComponent.CreateDynamicMaterialInstance` (`self.Mesh`) 0 null "None"))
  (bind _output_get (set `self.MaterialInstance` _returnvalue))
  (`MaterialInstanceDynamic.SetVectorParameterValue` _output_get "BodyColor" (`self.EnemyColor`)))