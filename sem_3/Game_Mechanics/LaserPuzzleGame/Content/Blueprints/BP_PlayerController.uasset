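; Player controller that handles cursor aiming and shooting for the controlled pawn.
; Both mouse axis events run a complex Visibility trace under the cursor and, on a hit, turn the control rotation to face that point using only the look-at yaw.
; The Shoot input casts the pawn to BP_PlayerCharacter and calls its Shoot function.
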(event `InputAxisKey|MouseX`
  (params (AxisValue :type "Float (single-precision)"))
  (bind (_hitresult _returnvalue) (`self.GetHitResultUnderCursorByChannel` "TraceTypeQuery1"))
  (bind (_returnvalue_roll _returnvalue_pitch _returnvalue_yaw) (`KismetMathLibrary.BreakRotator` (`KismetMathLibrary.FindLookAtRotation` (`self.K2_GetActorLocation` (`self.K2_GetPawn`)) (`.Location` (`GameplayStatics.BreakHitResult` _hitresult)))))
  ;[1 1 1] aiming
  (if _returnvalue :!label _label
    (`self.SetControlRotation` (`KismetMathLibrary.MakeRotator` 0.0 0.0 _returnvalue_yaw))))

(event `InputAxisKey|MouseY`
  (params (AxisValue :type "Float (single-precision)"))
  ;[1 1 1] aiming
  (goto _label))

(event `InputAction|Shoot`
  (params (Key :type "Key Structure"))
  (:`Pressed`
    (bind _asbp_player_character (cast `/Game/Blueprints/BP_PlayerCharacter` (`self.K2_GetPawn`)))
    (`/Game/Blueprints/BP_PlayerCharacter.Shoot` _asbp_player_character)))

(fn `UserConstructionScript`)