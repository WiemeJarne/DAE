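; BP_PlayerPawn is the player's pawn, moved directly each Tick from forward and right movement input on the world XY plane.
; The input vector's length is clamped to 1 to prevent faster diagonals, scaled by delta time and MovementSpeed, then applied as a swept world offset.
; Rotation is reset to zero every frame; an interpolated turn toward the movement direction is present but unconnected.
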(event `self.ReceiveTick`
  (params (DeltaSeconds :type "Float (single-precision)"))
  (`self.K2_AddActorWorldOffset` (* (* (`KismetMathLibrary.ClampVectorSize` (`KismetMathLibrary.MakeVector` (`self.GetInputAxisValue`) (`self.GetInputAxisValue`)) 0.0 1.0) DeltaSeconds) (`self.MovementSpeed`)) true)
  (`self.K2_SetActorRotation` (struct)))

(fn `UserConstructionScript`)