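; Player character Blueprint that carries a weapon, shows the game HUD and handles death and respawn.
; BeginPlay spawns BP_BaseWeapon, attaches it to the mesh's WeaponSocket and creates the HUD widget.
; Primary and secondary fire events forward to the weapon while the health component reports alive.
; On death it disables movement, stops firing, waits briefly, requests respawn from BP_GameMode, then destroys the weapon and itself.
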(event `self.ReceiveBeginPlay`
  (`parent.ReceiveBeginPlay`)
  (`|ExecutionSequence`
    (:`then_0`
      ;[1 1 1] spawn weapon
      (bind _returnvalue (`|SpawnActorFromClass` "/Game/Blueprints/BP_BaseWeapon.BP_BaseWeapon_C" (`SceneComponent.K2_GetComponentToWorld` (`self.GunSocket`)) "Undefined" "OverrideRootScale" null null))
      (bind _output_get (set `self.CurrentWeapon` _returnvalue))
      (`self.K2_AttachToComponent` _output_get (`self.Mesh`) "WeaponSocket" "SnapToTarget" "SnapToTarget" "KeepRelative" true))
    (:`then_1`
      ;[1 1 1] setup HUD
      (bind _returnvalue_2 (`|CreateWidget` "/Game/Blueprints/BPW_GameHUD.BPW_GameHUD_C"))
      (`UserWidget.AddToViewport` _returnvalue_2 0))))

(event `PrimaryFire`
  (params (IsStart :type Boolean :default true))
  (if (not (`/Game/Blueprints/BPC_Health.IsDead` (`self.BPC_Health`)))
    (bind _currentweapon (`self.CurrentWeapon`)
      (:`then`
        (`/Game/Blueprints/BP_BaseWeapon.FirePrimary` _currentweapon IsStart))
      (:`else`))))

(event `SecondaryFire`
  (params (IsStart :type Boolean :default true))
  (if (not (`/Game/Blueprints/BPC_Health.IsDead` (`self.BPC_Health`)))
    (bind _currentweapon (`self.CurrentWeapon`)
      (:`then`
        (`/Game/Blueprints/BP_BaseWeapon.FireSecondary` _currentweapon IsStart))
      (:`else`))))

(event `self.BPC_Health.OnDeath`
  (bind _currentweapon (`self.CurrentWeapon`))
  (`CharacterMovementComponent.DisableMovement` (`self.CharacterMovement`))
  (`/Game/Blueprints/BP_BaseWeapon.FirePrimary` _currentweapon false)
  (`/Game/Blueprints/BP_BaseWeapon.FireSecondary` _currentweapon false)
  (`KismetSystemLibrary.Delay` 3.0)
  ;[1 1 1] respawn
  (bind _asbp_game_mode (cast `/Game/Blueprints/BP_GameMode` (`GameplayStatics.GetGameMode`))
    (:`then`
      (`/Game/Blueprints/BP_GameMode.RespawnPlayer` _asbp_game_mode))
    (:`CastFailed`
      _))
  (`self.K2_DestroyActor` (`self.CurrentWeapon`))
  (`self.K2_DestroyActor` self))

(fn `UserConstructionScript`
  (`parent.UserConstructionScript`))