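; Enemy spawner actor that creates BP_EnemeyCharacter AI pawns when its Spawn event is called.
; Spawn counts living enemies in the level and skips spawning once the game mode's active-enemy cap is reached, falling back to a default cap if the cast fails.
; New enemies appear at a random point inside the spawn volume when UseSpawnVolume is set, otherwise at the actor's root.
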(event `Spawn`
  (bind _spawnvolume (`self.spawnVolume`))
  (bind (_asbp_game_mode _bsuccess) (cast `/Game/Blueprints/BP_GameMode` (`GameplayStatics.GetGameMode`) :!pure true))
  (bind _outactors (`GameplayStatics.GetAllActorsOfClass` "/Game/Blueprints/BP_EnemeyCharacter.BP_EnemeyCharacter_C"))
  (if (not (>= (`KismetArrayLibrary.Array_Length` _outactors) (select `bool` _bsuccess :`false` 5 :`true` (`/Game/Blueprints/BP_GameMode.MaxAmountOfActiveEnemies` _asbp_game_mode))))
    (`AIBlueprintHelperLibrary.SpawnAIFromClass` "/Game/Blueprints/BP_EnemeyCharacter.BP_EnemeyCharacter_C" null (select `bool` (`self.UseSpawnVolume`) :`false` (`SceneComponent.K2_GetComponentLocation` (`self.DefaultSceneRoot`)) :`true` (`KismetMathLibrary.RandomPointInBoundingBox` (`SceneComponent.K2_GetComponentLocation` _spawnvolume) (`BoxComponent.GetScaledBoxExtent` _spawnvolume))) (`SceneComponent.K2_GetComponentRotation` (`self.DefaultSceneRoot`)) false null)))

(fn `UserConstructionScript`)