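; BPC_Health is a Blueprint health component that tracks current health against a maximum and signals death.
; Health resets to max on BeginPlay, and DoDamage clamps it between zero and max, so negative amounts heal.
; DoDamage returns whether the owner is dead and calls OnDeath only when that hit lowered health to zero, avoiding repeat triggers.
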(event `ResetHealth`
  (set `self.CurrentHealth` (`self.maxHealth`)))

(event `self.ReceiveBeginPlay`
  (`self.ResetHealth`))

(fn `DoDamage`
  (params (amount :type "Float (double-precision)"))
  (returns (isDead :type Boolean))
  (locals (OriginalHealth :type "Float (double-precision)"))
  (bind _isdead (`self.IsDead`))
  ;[1 1 1] cache original health value
  (set `local.OriginalHealth` (`self.CurrentHealth`))
  (bind _output_get (set `self.CurrentHealth` (`KismetMathLibrary.FClamp` (- (`self.CurrentHealth`) amount) 0.0 (`self.maxHealth`))))
  ;[1 1 1] did this DoDamage cause the health to change and drop to 0?
  (if (and _isdead (> (`local.OriginalHealth`) _output_get))
    (`self.OnDeath`))
  (return _isdead))

(fn `GetHealthPercentage`
  (returns (healthPercentage :type "Float (double-precision)"))
  (return (/ (`self.CurrentHealth`) (`self.maxHealth`))))

(fn `IsDead`
  (returns (IsDead :type Boolean))
  (return (== (`self.GetHealthPercentage`) 0.0)))