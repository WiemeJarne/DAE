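; Enemy character that damages the player on contact and adds to the game mode score when killed.
; Overlapping the player starts a looping timer that damages their health component, cleared when the overlap ends.
; On death it disables movement and collision, screams and destroys itself after a delay.
; Dynamic materials set the body color and tint a second slot from a color curve driven by health percentage, updated every tick.
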(event `self.ReceiveActorBeginOverlap`
  (params (OtherActor :type "Actor Object Reference"))
  (`parent.ReceiveActorBeginOverlap` OtherActor)
  (bind _asbp_player_character (cast `/Game/Blueprints/BP_PlayerCharacter` OtherActor))
  (set `self.CurrentPlayerCharacter` _asbp_player_character)
  (`KismetSystemLibrary.K2_SetTimerDelegate` (delegate `DamageCurrentPlayerTarget`) (`self.AttackInterval`) true))

(event `DamageCurrentPlayerTarget`
  (bind _currentplayercharacter (`self.CurrentPlayerCharacter`)
    (:`then`
      (`/Game/Blueprints/BPC_Health.DoDamage` (`/Game/Blueprints/BP_BaseCharacter.BPC_Health` _currentplayercharacter) (`self.DamageAmount`)))
    (:`else`)))

(event `self.ReceiveActorEndOverlap`
  (params (OtherActor :type "Actor Object Reference"))
  (if (== OtherActor (`self.CurrentPlayerCharacter`))
    (`KismetSystemLibrary.K2_ClearTimer` null "DamageCurrentPlayerTarget")))

(event `self.BPC_Health.OnDeath`
  (bind _capsulecomponent (`self.CapsuleComponent`))
  (`|ExecutionSequence`
    (:`then_0`
      (bind _asbp_game_mode (cast `/Game/Blueprints/BP_GameMode` (`GameplayStatics.GetGameMode`)))
      (`/Game/Blueprints/BP_GameMode.IncrementScore` _asbp_game_mode (`self.ScoreAmount`)))
    (:`then_1`
      (`CharacterMovementComponent.DisableMovement` (`self.CharacterMovement`))
      (`KismetSystemLibrary.K2_ClearTimer` null "DamageCurrentPlayerTarget")
      (`PrimitiveComponent.SetCollisionEnabled` (`self.DamageZone`) "NoCollision")
      (`PrimitiveComponent.SetCollisionResponseToChannel` _capsulecomponent "ECC_WorldStatic" "ECR_Ignore")
      (`PrimitiveComponent.SetCollisionResponseToChannel` _capsulecomponent "ECC_Pawn" "ECR_Ignore")
      (`GameplayStatics.SpawnSoundAttached` "/Game/Audio/WilhelmScream.WilhelmScream" (`self.Mesh`) "None" (0.0 0.0 0.0) (struct) "KeepRelativeOffset" false 1.0 1.0 0.0 null null)
      (`KismetSystemLibrary.Delay` 3.0)
      (`self.K2_DestroyActor`))))

(event `self.ReceiveTick`
  (params (DeltaSeconds :type "Float (single-precision)"))
  (bind _bpc_health (`self.BPC_Health`))
  (`parent.ReceiveTick` DeltaSeconds)
  (bind _healthmaterialinstance (`self.HealthMaterialInstance`)
    (:`then`
      (`MaterialInstanceDynamic.SetVectorParameterValue` _healthmaterialinstance "color" (select `bool` (`KismetSystemLibrary.IsValid` _bpc_health) :`false` (struct :`R` 0.824993 :`G` 0.921875 :`B` 0.187256 :`A` 1.0) :`true` (`CurveLinearColor.GetLinearColorValue` (`self.HleathColorCurve`) (`/Game/Blueprints/BPC_Health.GetHealthPercentage` _bpc_health)))))
    (:`else`)))

(fn `UserConstructionScript`
  (bind _bpc_health (`self.BPC_Health`))
  (`parent.UserConstructionScript`)
  (bind _returnvalue (`PrimitiveComponent.CreateDynamicMaterialInstance` (`self.Mesh`) 0 null "None"))
  (bind _output_get (set `self.MaterialInstance` _returnvalue))
  (`MaterialInstanceDynamic.SetVectorParameterValue` _output_get "BodyColor" (`self.EnemyColor`))
  (bind _returnvalue_2 (`PrimitiveComponent.CreateDynamicMaterialInstance` (`self.Mesh`) 1 null "None"))
  (bind _output_get_2 (set `self.HealthMaterialInstance` _returnvalue_2))
  (`MaterialInstanceDynamic.SetVectorParameterValue` _output_get_2 "color" (select `bool` (`KismetSystemLibrary.IsValid` _bpc_health) :`false` (struct :`R` 0.824993 :`G` 0.921875 :`B` 0.187256 :`A` 1.0) :`true` (`CurveLinearColor.GetLinearColorValue` (`self.HleathColorCurve`) (`/Game/Blueprints/BPC_Health.GetHealthPercentage` _bpc_health)))))