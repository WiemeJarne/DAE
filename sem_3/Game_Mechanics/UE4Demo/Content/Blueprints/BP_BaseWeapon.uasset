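; BP_BaseWeapon is a base weapon Blueprint that handles held automatic primary fire and a stubbed secondary fire.
; FirePrimary spawns a projectile immediately on press, then repeats on a looping timer derived from PrimaryFireRate, behind a DoOnce that resets when release clears the timer.
; Projectiles use PrimaryProjectileClass and spawn at the FireSocket's world transform.
; FireSecondary only prints a debug string.
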(event `FirePrimary`
  (params (IsStart :type Boolean :default true))
  (if IsStart
    (`/Engine/EditorBlueprintResources/StandardMacros.DoOnce` false :!label _label
      (:`Completed`
        (`self.SpawnPrimaryProjectile`)
        (`KismetSystemLibrary.K2_SetTimerDelegate` (delegate `SpawnPrimaryProjectile`) (/ 1.0 (`self.PrimaryFireRate`)) true)))
    (else
      (`KismetSystemLibrary.K2_ClearTimer` null "SpawnPrimaryProjectile")
      (goto _label :!via `Reset`))))

(event `SpawnPrimaryProjectile`
  (`|SpawnActorFromClass` (`self.PrimaryProjectileClass`) (`SceneComponent.K2_GetComponentToWorld` (`self.FireSocket`)) "Undefined" "OverrideRootScale" null null))

(event `FireSecondary`
  (params (IsStart :type Boolean))
  (if IsStart
    (`KismetSystemLibrary.PrintString` "secondary")))

(fn `UserConstructionScript`)