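; Player controller for world-axis movement, twin-stick or mouse aiming, and forwarding primary and secondary fire to BP_PlayerCharacter.
; Mouse motion enables cursor aim, turning control yaw toward a visibility-trace hit and placing a lazily spawned BP_MouseAimTarget there.
; Look-axis input sets control rotation only while mouse aim is off.
; After MovementAimTimeDelay without aim input, movement handlers clear mouse aim, hide the target and face the movement direction.
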(event `InputAxis|MovementForward`
  (params (AxisValue :type "Float (single-precision)"))
  (bind _returnvalue (`Pawn.GetLastMovementInputVector` (`self.K2_GetPawn`)))
  (bind (_returnvalue_roll _returnvalue_pitch _returnvalue_yaw) (`KismetMathLibrary.BreakRotator` (`KismetMathLibrary.Conv_VectorToRotator` _returnvalue)))
  (`Pawn.AddMovementInput` (`self.K2_GetPawn`) (1.0 0.0 0.0) AxisValue false)
  (if (>= (- (`KismetSystemLibrary.GetGameTimeInSeconds`) (`self.LastAimInputTime`)) (`self.MovementAimTimeDelay`)) :!label _label
    (set `self.UseMouseAim` false)
    (bind _currentmouseaimtarget (`self.CurrentMouseAimTarget`)
      (:`then`
        (`self.SetActorHiddenInGame` _currentmouseaimtarget true))
      (:`else`
        _))
    (if (> (`KismetMathLibrary.VSize` _returnvalue) 0.0)
      (`self.SetControlRotation` (`KismetMathLibrary.MakeRotator` _returnvalue_roll 0.0 _returnvalue_yaw)))))

(event `InputAxis|MovementRight`
  (params (AxisValue :type "Float (single-precision)"))
  (`Pawn.AddMovementInput` (`self.K2_GetPawn`) (0.0 1.0 0.0) AxisValue false)
  (goto _label))

(event `InputAxis|LookUp`
  (params (AxisValue :type "Float (single-precision)"))
  ;[1 1 1] aiming
  (if (not (`self.UseMouseAim`)) :!label _label_2
    (bind _returnvalue (`KismetMathLibrary.MakeVector` AxisValue (stale `InputAxis|LookRight` AxisValue)))
    (if (> (`KismetMathLibrary.VSize` _returnvalue) 0.25)
      (set `self.UseMouseAim` false)
      (bind _currentmouseaimtarget (`self.CurrentMouseAimTarget`)
        (:`then`
          (`self.SetActorHiddenInGame` _currentmouseaimtarget true))
        (:`else`
          _))
      (`self.SetControlRotation` (`KismetMathLibrary.Conv_VectorToRotator` _returnvalue))
      (set `self.LastAimInputTime` (`KismetSystemLibrary.GetGameTimeInSeconds`)))))

(event `self.ReceiveTick`
  (params (DeltaSeconds :type "Float (single-precision)")))

(event `InputAxis|LookRight`
  (params (AxisValue :type "Float (single-precision)"))
  ;[1 1 1] aiming
  (goto _label_2))

(event `InputAction|FirePrimary`
  (params (Key :type "Key Structure"))
  (bind _returnvalue (`self.K2_GetPawn`))
  (:`Pressed`
    (bind _asbp_player_character (cast `/Game/Blueprints/BP_PlayerCharacter` _returnvalue))
    (`/Game/Blueprints/BP_PlayerCharacter.PrimaryFire` _asbp_player_character true))
  (:`Released`
    (bind _asbp_player_character_2 (cast `/Game/Blueprints/BP_PlayerCharacter` _returnvalue))
    (`/Game/Blueprints/BP_PlayerCharacter.PrimaryFire` _asbp_player_character_2 false)))

(event `InputAction|FireSecondary`
  (params (Key :type "Key Structure"))
  (bind _returnvalue (`self.K2_GetPawn`))
  (:`Pressed`
    (bind _asbp_player_character (cast `/Game/Blueprints/BP_PlayerCharacter` _returnvalue))
    (`/Game/Blueprints/BP_PlayerCharacter.SecondaryFire` _asbp_player_character true))
  (:`Released`
    (bind _asbp_player_character_2 (cast `/Game/Blueprints/BP_PlayerCharacter` _returnvalue))
    (`/Game/Blueprints/BP_PlayerCharacter.SecondaryFire` _asbp_player_character_2 false)))

(event `InputAxisKey|MouseX`
  (params (AxisValue :type "Float (single-precision)"))
  (bind (_hitresult _returnvalue) (`self.GetHitResultUnderCursorByChannel` "TraceTypeQuery1"))
  (bind (_bblockinghit _binitialoverlap _time _distance _location) (`GameplayStatics.BreakHitResult` _hitresult))
  (bind (_returnvalue_roll _returnvalue_pitch _returnvalue_yaw) (`KismetMathLibrary.BreakRotator` (`KismetMathLibrary.FindLookAtRotation` (`self.K2_GetActorLocation` (`self.K2_GetPawn`)) _location)))
  ;[1 1 1] aiming
  (`|ExecutionSequence` :!label _label_3
    (:`then_0`
      (if (> (`KismetMathLibrary.VSize` (`KismetMathLibrary.MakeVector` AxisValue (stale `InputAxisKey|MouseY` AxisValue))) 0.25)
        (set `self.UseMouseAim` true)
        (set `self.LastAimInputTime` (`KismetSystemLibrary.GetGameTimeInSeconds`))))
    (:`then_1`
      (if (`self.UseMouseAim`)
        (`|ExecutionSequence`
          (:`then_0`
            (`self.CurrentMouseAimTarget`
              (:`then`)
              (:`else`
                (bind _returnvalue_2 (`|SpawnActorFromClass` "/Game/Blueprints/BP_MouseAimTarget.BP_MouseAimTarget_C" (`KismetMathLibrary.MakeTransform` (0.0 0.0 0.0)) "Undefined" "OverrideRootScale" null null))
                (set `self.CurrentMouseAimTarget` _returnvalue_2))))
          (:`then_1`
            (if _returnvalue
              (`self.SetControlRotation` (`KismetMathLibrary.MakeRotator` 0.0 0.0 _returnvalue_yaw))
              (bind _currentmouseaimtarget (`self.CurrentMouseAimTarget`)
                (:`then`
                  (`self.SetActorHiddenInGame` _currentmouseaimtarget false)
                  (`self.K2_SetActorLocation` _currentmouseaimtarget _location false false))
                (:`else`)))))))))

(event `InputAxisKey|MouseY`
  (params (AxisValue :type "Float (single-precision)"))
  ;[1 1 1] aiming
  (goto _label_3))

(fn `UserConstructionScript`)