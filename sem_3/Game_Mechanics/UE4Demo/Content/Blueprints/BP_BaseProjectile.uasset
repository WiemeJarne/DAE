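; Base projectile actor that damages what it hits, on either an actor overlap or a Collision component hit.
; Both events feed ProcessCollision, which skips actors carrying the ignore tag and applies damage through the BPI_Damagable interface, falling back to a BPC_Health component.
; A successful damage hit plays an impact sound and particle effect, then destroys the projectile; other contacts leave it alive.
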(event `self.ReceiveActorBeginOverlap`
  (params (OtherActor :type "Actor Object Reference"))
  (`self.ProcessCollision` OtherActor))

(event `self.Collision.OnComponentHit`
  (params (HitComponent :type "PrimitiveComponent Object Reference") (OtherActor :type "Actor Object Reference") (OtherComp :type "PrimitiveComponent Object Reference") (NormalImpulse :type "Vector Structure") (Hit :type "HitResult Structure (by ref)"))
  (`self.ProcessCollision` OtherActor))

(fn `ProcessCollision`
  (params (OtherActor :type "Actor Object Reference"))
  (bind _returnvalue (`self.GetComponentByClass` OtherActor "/Game/Blueprints/BPC_Health.BPC_Health_C"))
  (bind _collision (`self.Collision`))
  ;[1 1 1] check if the projectile hit an actor
  (`/Engine/EditorBlueprintResources/StandardMacros.IsValid` OtherActor
    (:`Is Valid`
      ;[1 1 1] check if the target doesn't have a matching ignore tag
      (if (not (`self.ActorHasTag` OtherActor (`self.IgnoreTag`)))
        ;[1 1 1] BPI_Damageable
        (if (`KismetSystemLibrary.DoesImplementInterface` OtherActor "/Game/Blueprints/BPI_Damagable.BPI_Damagable_C")
          (message `/Game/Blueprints/BPI_Damagable.DoDamage` OtherActor (`self.Damage`))
          (else
            ;[1 1 1] get and check if there is a health component
            (`/Engine/EditorBlueprintResources/StandardMacros.IsValid` _returnvalue
              (:`Is Valid`
                ;[1 1 1] damage
                (`/Game/Blueprints/BPC_Health.DoDamage` _returnvalue (`self.Damage`))))))
        (`GameplayStatics.SpawnSoundAttached` "/Game/Audio/234082__211redman112__lasgun-impact.234082__211redman112__lasgun-impact" (`self.Collision`) "None" (0.0 0.0 0.0) (struct) "KeepRelativeOffset" false 1.0 1.0 0.0 null null)
        (`GameplayStatics.SpawnEmitterAtLocation` "/Game/Particles/P_ProjectileImplact.P_ProjectileImplact" (`SceneComponent.K2_GetComponentLocation` _collision) (`SceneComponent.K2_GetComponentRotation` _collision))
        (`self.K2_DestroyActor`)))))

(fn `UserConstructionScript`)